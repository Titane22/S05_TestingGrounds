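; AI controller for guard NPCs that starts the GuardBehavior behavior tree with the PatrolData blackboard.
; Perception updates on sensing an actor without the "Enemy" tag set the controlled BP_Character aiming and store player pawn 0 as the blackboard Enemy.
; Other valid updates stop aiming and clear that key.
; FindPatrolRoute writes the controlled ThirdPersonCharacter's first patrol point to the Waypoint key of a supplied blackboard.
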(event OnTargetPerceptionUpdated(AIPerception)
  (params (Actor :type Actor%20Object%20Reference) (Stimulus :type AI%20Stimulus%20Structure))
  (bind _enemy (Variables|Default|GetEnemy))
  (bind _blackboard_comp (Variables|Default|GetBlackboard%20Comp))
  (Utilities|IsValid Actor
    (:Is%20Valid
      (bind _asbp_character (Utilities|Casting|CastToBP_Character (Pawn|GetControlledPawn)))
      (if (and (not (Actor|ActorHasTag Actor "Enemy")) (.bSuccessfullySensed (Utilities|Struct|BreakAIStimulus Stimulus)))
        (Variables|/Game/Character/Characters/BP_Character.BP_Character_C|SetAiming _asbp_character true)
        (AI|Components|Blackboard|SetValueasObject _blackboard_comp _enemy (Game|Player|GetPlayerPawn 0))
        (else
          (Variables|/Game/Character/Characters/BP_Character.BP_Character_C|SetAiming _asbp_character false)
          (AI|Components|Blackboard|ClearValue _blackboard_comp _enemy))))))

(event EventBeginPlay
  (bind _blackboardcomponent (Class|AIController|UseBlackboard "/Game/Character/AI/PatrolData.PatrolData"))
  (AI|RunBehaviorTree "/Game/Character/AI/GuardBehavior.GuardBehavior")
  (Variables|Default|SetBlackboard%20Comp _blackboardcomponent))

(fn ConstructionScript)

(fn FindPatrolRoute
  (params (Waypoint :type Blackboard%20Component%20Object%20Reference))
  (bind _asthird_person_character (Utilities|Casting|CastToThirdPersonCharacter (Pawn|GetControlledPawn)))
  (AI|Components|Blackboard|SetValueasObject Waypoint (Utilities|Name|MakeLiteralName "Waypoint") (Utilities|Array|Get(acopy) (Variables|/Game/Trash/ThirdPersonCharacter.ThirdPersonCharacter_C|GetPatrol%20Points _asthird_person_character))))