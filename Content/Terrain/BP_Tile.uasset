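; Terrain tile for an infinite-terrain mode that scatters containers, canisters, sandbags, boxes and rocks through PlaceActors on BeginPlay.
; The player entering LockingVolume opens the barrier and turns it green; leaving relocks it red and asks InfiniteTerrainGameMode to spawn another tile.
; DestroyVolume removes the tile when the player overlaps it, and GetAttachLocation exposes the Arrow's world transform as an attach point.
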(event OnComponentBeginOverlap(LockingVolume)
  (params (OverlappedComponent :type Primitive%20Component%20Object%20Reference) (OtherActor :type Actor%20Object%20Reference) (OtherComp :type Primitive%20Component%20Object%20Reference) (OtherBodyIndex :type Integer) (bFromSweep :type Boolean) (SweepResult :type Hit%20Result%20Structure%20%28by%20ref%29))
  (Utilities|IsPlayerActor OtherActor
    (:NewParam
      (CallFunction|Unlock))))

(event OnComponentEndOverlap(LockingVolume)
  (params (OverlappedComponent :type Primitive%20Component%20Object%20Reference) (OtherActor :type Actor%20Object%20Reference) (OtherComp :type Primitive%20Component%20Object%20Reference) (OtherBodyIndex :type Integer))
  (Utilities|IsPlayerActor OtherActor
    (:NewParam
      (CallFunction|Lock)
      (bind _asinfinite_terrain_game_mode (Utilities|Casting|CastToInfiniteTerrainGameMode (Game|GetGameMode)))
      (Default|SpawnTile _asinfinite_terrain_game_mode))))

(event OnComponentBeginOverlap(DestroyVolume)
  (params (OverlappedComponent :type Primitive%20Component%20Object%20Reference) (OtherActor :type Actor%20Object%20Reference) (OtherComp :type Primitive%20Component%20Object%20Reference) (OtherBodyIndex :type Integer) (bFromSweep :type Boolean) (SweepResult :type Hit%20Result%20Structure%20%28by%20ref%29))
  (Utilities|IsPlayerActor OtherActor
    (:NewParam
      (Actor|DestroyActor))))

(event EventBeginPlay
  (CallFunction|Lock)
  (Class|Tile|PlaceActors "/Game/Terrain/Props/BP_Container.BP_Container_C" 1 3 1000)
  (Class|Tile|PlaceActors "/Game/Terrain/Props/BP_Canister.BP_Canister_C" 1 7 100)
  (Class|Tile|PlaceActors "/Game/Terrain/Props/BP_SandBag.BP_SandBag_C" 0 1 150)
  (Class|Tile|PlaceActors "/Game/Terrain/Props/BP_Box.BP_Box_C" 2 4 100)
  (Class|Tile|PlaceActors "/Game/Terrain/Props/BP_Rock1.BP_Rock1_C" 0 4 300)
  (Class|Tile|PlaceActors "/Game/Terrain/Props/BP_Rock2.BP_Rock2_C" 0 4 300)
  (Class|Tile|PlaceActors "/Game/Terrain/Props/BP_Rock3.BP_Rock3_C" 0 4 300))

(fn ConstructionScript)

(fn GetAttachLocation
  (return (Transformation|GetWorldTransform (Variables|Default|GetArrow))))

(fn Unlock
  (Collision|SetCollisionEnabled (Variables|Default|GetBarrier) "NoCollision")
  (Rendering|Material|SetMaterial (Variables|Default|GetBarrier) 0 "/Game/Terrain/Materials/GreenBarrier.GreenBarrier"))

(fn Lock
  (bind _barrier (Variables|Default|GetBarrier))
  (Collision|SetCollisionEnabled _barrier "QueryAndPhysics")
  (Rendering|Material|SetMaterial _barrier 0 "/Game/Terrain/Materials/RedBarrier.RedBarrier"))